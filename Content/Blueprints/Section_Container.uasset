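; Section_Container is a Blueprint that appears to be an unfinished container for Section child actors.
; Its construction script loops over the direct children of DefaultSceneRoot, casts each to ChildActorComponent, and prints a debug message when the component's own class equals Section.
; The node that adds to the Sections array is disconnected, so nothing is collected, and the event graph holds only disabled default events.
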(fn `UserConstructionScript`
  (for _array_element (`SceneComponent.GetChildrenComponents` (`self.DefaultSceneRoot`) false)
    (bind _aschild_actor_component (cast `ChildActorComponent` _array_element))
    (if (== (`GameplayStatics.GetObjectClass` _aschild_actor_component) "/Game/Blueprints/Section.Section_C")
      (`KismetSystemLibrary.PrintString` "Hello"))))