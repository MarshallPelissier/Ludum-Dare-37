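; Light source Blueprint that switches the visibility of the directional light components under its shared root, separately for construction and gameplay.
; When Off is set, the construction script loops over the root's children and toggles each directional light's visibility, flipping it rather than forcing it hidden.
; On BeginPlay, the same child loop sets each directional light's visibility to OnIngame.
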(event `self.ReceiveBeginPlay`
  (bind _sharedroot (`self.SharedRoot`))
  (for _index (range (`SceneComponent.GetNumChildrenComponents` _sharedroot))
    (bind _asdirectional_light_component (cast `DirectionalLightComponent` (`SceneComponent.GetChildComponent` _sharedroot _index)))
    (`SceneComponent.SetVisibility` _asdirectional_light_component (`self.On_ingame`) false)))

(fn `UserConstructionScript`
  (bind _sharedroot (`self.SharedRoot`))
  (if (`self.Off`)
    (for _index (range (`SceneComponent.GetNumChildrenComponents` _sharedroot))
      (bind _asdirectional_light_component (cast `DirectionalLightComponent` (`SceneComponent.GetChildComponent` _sharedroot _index)))
      (`SceneComponent.ToggleVisibility` _asdirectional_light_component false))))