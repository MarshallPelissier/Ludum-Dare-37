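; Section controller that applies one of four level presets to every Section_Container actor in the world.
; The construction script caches the containers with GetAllActorsOfClass.
; Each level event sets size and rate ranges plus Launch and Osc values, then pushes them to all containers and resets their sections.
; BeginPlay applies the current values, while EvenLevelSelect switches presets by number, falling back to Level 1.
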(event `self.ReceiveBeginPlay`
  (`self.Event SetContainers`)
  (`self.Event ResetContainers`))

(event `Event ResetContainers`
  (for _array_element (`self.SectionContainers`)
    (`/Game/Blueprints/Section_Container.Event ResetSections` _array_element)))

(event `Event SetContainers`
  (for _array_element (`self.SectionContainers`)
    (`/Game/Blueprints/Section_Container.Event ContainerValues` _array_element (`self.SizeMin`) (`self.SizeMax`) (`self.RateMin`) (`self.RateMax`) (`self.Launch`) (`self.Osc`))))

(event `Event Level1`
  (set `self.SizeMin` 1.0)
  (set `self.SizeMax` 1.0)
  (set `self.RateMin` 3.0)
  (set `self.RateMax` 10.0)
  (set `self.Launch` 9)
  (set `self.Osc` 5)
  (`self.Event SetContainers` :!label _label)
  (`self.Event ResetContainers`))

(event `Event Level2`
  (set `self.SizeMin` 1.0)
  (set `self.SizeMax` 2.0)
  (set `self.RateMin` 2.0)
  (set `self.RateMax` 8.0)
  (set `self.Launch` 7)
  (set `self.Osc` 4)
  (goto _label))

(event `Event Level3`
  (set `self.SizeMin` 1.0)
  (set `self.SizeMax` 3.0)
  (set `self.RateMin` 2.0)
  (set `self.RateMax` 6.0)
  (set `self.Launch` 5)
  (set `self.Osc` 3)
  (goto _label))

(event `Event Level4`
  (set `self.SizeMin` 1.0)
  (set `self.SizeMax` 4.0)
  (set `self.RateMin` 0.0)
  (set `self.RateMax` 5.0)
  (set `self.Launch` 4)
  (set `self.Osc` 3)
  (goto _label))

(event `Even LevelSelect`
  (params (level :type Integer))
  (switch `int` level
    (:`Default`
      (`self.Event Level1` :!label _label_2))
    (:`0`
      (goto _label_2))
    (:`1`
      (goto _label_2))
    (:`2`
      (`self.Event Level2`))
    (:`3`
      (`self.Event Level3`))
    (:`4`
      (`self.Event Level4`))))

(fn `UserConstructionScript`
  (bind _outactors (`GameplayStatics.GetAllActorsOfClass` "/Game/Blueprints/Section_Container.Section_Container_C"))
  (set `self.SectionContainers` _outactors))