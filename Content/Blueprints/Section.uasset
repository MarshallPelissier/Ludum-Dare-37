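; Level section actor that randomizes itself at BeginPlay into a static or oscillating piece, with a minority keeping a projectile launcher instead of a cap.
; A timeline moves the container to a random height, then a second timeline optionally oscillates it.
; Launchers fire upward after random delays, looping when static or triggered by accumulated timeline progress when oscillating.
; Non-character box overlaps can halt positioning or flip oscillation direction via FlipFlops.
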(event `self.ReceiveBeginPlay`
  (bind _randstream (`self.RandStream`))
  (bind _returnvalue (`KismetMathLibrary.RandomFloatInRangeFromStream` 100.0 500.0 _randstream))
  (bind _returnvalue_2 (`KismetMathLibrary.FTrunc` _returnvalue))
  (`KismetMathLibrary.SeedRandomStream` (`self.RandStream`))
  (`self.Event StartingPosition`)
  (set `self.MaxOscilation` (* (`KismetMathLibrary.SelectInt` -1 1 (`KismetMathLibrary.RandomBoolFromStream` _randstream)) _returnvalue))
  (`|ExecutionSequence`
    (:`then_0`
      (switch `int` (mod _returnvalue_2 4)
        (:`0`
          (set `self.Oscilate` true :!label _label))
        (:`1`
          (goto _label))
        (:`2`
          (set `self.Oscilate` false :!label _label_2))
        (:`3`
          (goto _label_2))))
    (:`then_1`
      (switch `int` (mod _returnvalue_2 10)
        (:`0`
          (set `self.Shooter` true :!label _label_3)
          (`ActorComponent.K2_DestroyComponent` (`self.Section_Cap_2d5x2d5`)))
        (:`1`
          (goto _label_3))
        (:`2`
          (`ActorComponent.K2_DestroyComponent` (`self.Launcher_2d5x2x5`) :!label _label_4))
        (:`3`
          (goto _label_4))
        (:`4`
          (goto _label_4))
        (:`5`
          (goto _label_4))
        (:`6`
          (goto _label_4))
        (:`7`
          (goto _label_4))
        (:`8`
          (goto _label_4))
        (:`9`
          (goto _label_4))))))

(event `Event FireProjectile`
  (params (Osc :type Boolean))
  (bind (_returnvalue_x _returnvalue_y _returnvalue_z) (`KismetMathLibrary.BreakVector` (`SceneComponent.K2_GetComponentLocation` (`self.Launcher_2d5x2x5`))))
  (`KismetSystemLibrary.Delay` (`KismetMathLibrary.RandomFloatInRangeFromStream` 4.0 10.0 (`self.RandStream`)))
  (`|SpawnActorFromClass` "/Game/FirstPersonBP/Blueprints/FirstPersonProjectile.FirstPersonProjectile_C" (`KismetMathLibrary.MakeTransform` (`KismetMathLibrary.MakeVector` _returnvalue_x _returnvalue_y (+ _returnvalue_z 10.0)) (`KismetMathLibrary.Conv_VectorToRotator` (`KismetMathLibrary.GetUpVector` (`self.K2_GetActorRotation`)))) "Undefined" "OverrideRootScale")
  (if (not Osc)
    (`self.Event FireProjectile` false)))

(event `Event StartingPosition`
  (bind _section_container_2d5x10 (`self.Section_Container_2d5x10`))
  (bind (_relativelocation_x _relativelocation_y _relativelocation_z) (`KismetMathLibrary.BreakVector` (`SceneComponent.RelativeLocation` _section_container_2d5x10)))
  (set `self.Positioning` true)
  (bind _output_get (set `self.NewZ` (`KismetMathLibrary.RandomFloatInRangeFromStream` 0.0 (`self.MaxMovement`) (`self.RandStream`))))
  (bind _output_get_2 (set `self.StartZ` _relativelocation_z))
  (bind (_direction _driver) (`Timeline|Timeline_0` :!via `PlayFromStart` :!label _label_5)
    (:`Update`
      (`SceneComponent.K2_SetRelativeLocation` _section_container_2d5x10 (`KismetMathLibrary.MakeVector` 0.0 0.0 (`KismetMathLibrary.Lerp` _output_get_2 _output_get _driver)) false false))
    (:`Finished`
      (if (`self.Oscilate`) :!label _label_6
        (set `self.Positioning` false)
        (`self.Event Oscilate`)
        (else
          (set `self.Positioning` false)
          (set `self.Done` true)
          (if (`self.Shooter`)
            (`self.Event FireProjectile` (`self.Oscilate`))))))))

(event `Event Oscilate`
  (bind _section_container_2d5x10 (`self.Section_Container_2d5x10`))
  (bind (_relativelocation_x _relativelocation_y _relativelocation_z) (`KismetMathLibrary.BreakVector` (`SceneComponent.RelativeLocation` _section_container_2d5x10)))
  (`TimelineComponent.SetPlayRate` (`self.Timeline_1`) (`KismetMathLibrary.RandomFloatInRangeFromStream` 0.1 0.5 (`self.RandStream`)))
  (bind _output_get (set `self.NewO` (+ _relativelocation_z (`self.MaxOscilation`))))
  (bind _output_get_2 (set `self.StartZ` _relativelocation_z))
  (bind (_direction _driver) (`Timeline|Timeline_1` :!via `PlayFromStart` :!label _label_7)
    (:`Update`
      (set `self.ShotCount` (+ (`self.ShotCount`) _driver))
      (`SceneComponent.K2_SetRelativeLocation` _section_container_2d5x10 (`KismetMathLibrary.MakeVector` 0.0 0.0 (`KismetMathLibrary.Lerp` _output_get_2 _output_get _driver)) false false)
      (if (`self.Shooter`)
        (if (> (`self.ShotCount`) (* (`self.NewO`) 0.3))
          (set `self.ShotCount` 0.0)
          (`self.Event FireProjectile` (`self.Oscilate`)))))))

(event `self.Box.OnComponentBeginOverlap`
  (params (OverlappedComponent :type "PrimitiveComponent Object Reference") (OtherActor :type "Actor Object Reference") (OtherComp :type "PrimitiveComponent Object Reference") (OtherBodyIndex :type Integer) (bFromSweep :type Boolean) (SweepResult :type "HitResult Structure (by ref)"))
  (cast `Character` OtherActor
    (:`CastFailed`
      (if (`self.Done`)
        _
        (elif (`self.Positioning`)
          (`/Engine/EditorBlueprintResources/StandardMacros.FlipFlop`
            (:`A`
              (`|ExecutionSequence`
                (:`then_0`
                  (goto _label_5 :!via `Stop`))
                (:`then_1`
                  (goto _label_6)))))
          (else
            (`/Engine/EditorBlueprintResources/StandardMacros.FlipFlop`
              (:`A`
                (goto _label_7 :!via `Reverse`))
              (:`B`
                (goto _label_7)))))))))

(event `self.Box.OnComponentEndOverlap`
  (params (OverlappedComponent :type "PrimitiveComponent Object Reference") (OtherActor :type "Actor Object Reference") (OtherComp :type "PrimitiveComponent Object Reference") (OtherBodyIndex :type Integer)))

(fn `UserConstructionScript`
  (`TimelineComponent.SetPlayRate` (`self.Timeline_0`) (`self.Timeline_0PlayRate`)))