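; FinishButton is the level exit, a button that turns green when opened and finishes the run when a Character overlaps its box.
; Finishing resets the button, moves Level up on success or down on death within a clamped range, and destroys all FirstPersonProjectile actors.
; The new Level then drives difficulty selection on SectionController and key spawning on KeyController.
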(event `Event Open`
  (set `self.Open` true)
  (`PrimitiveComponent.SetMaterial` (`self.p_2x20_vertical`) 0 "/Game/Materials/Emissive/Emissive_Green.Emissive_Green"))

(event `Event Reset`
  (set `self.Open` false)
  (`PrimitiveComponent.SetMaterial` (`self.p_2x20_vertical`) 0 "/Game/Materials/Base2.Base2"))

(event `self.Box.OnComponentBeginOverlap`
  (params (OverlappedComponent :type "PrimitiveComponent Object Reference") (OtherActor :type "Actor Object Reference") (OtherComp :type "PrimitiveComponent Object Reference") (OtherBodyIndex :type Integer) (bFromSweep :type Boolean) (SweepResult :type "HitResult Structure (by ref)"))
  (if (`self.Open`)
    (cast `Character` OtherActor)
    (`self.Event Finished` false)))

(event `Event Finished`
  (params (Died :type Boolean))
  (bind _level (`self.Level`))
  (`self.Event Reset`)
  (bind _output_get (set `self.Level` (`KismetMathLibrary.Clamp` (`KismetMathLibrary.SelectInt` (- _level 1) (+ _level 1) Died) 0 4)))
  (bind _outactors (`GameplayStatics.GetAllActorsOfClass` "/Game/FirstPersonBP/Blueprints/FirstPersonProjectile.FirstPersonProjectile_C"))
  (for _array_element _outactors
    (`self.K2_DestroyActor` _array_element))
  (`self.Event SetDifficulty` _output_get)
  (`/Game/Blueprints/Key_Control.Event SpawnKeys` (`self.KeyController`) _output_get))

(event `Event SetDifficulty`
  (params (Level :type Integer))
  (`/Game/Blueprints/Section_Controller.Even LevelSelect` (`self.SectionController`) (`KismetMathLibrary.Clamp` Level 1 4)))

(fn `UserConstructionScript`)