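; Key puzzle controller that scatters key projectiles within a configurable volume and opens its linked Finish once all are removed.
; SpawnKeys maps a clamped input to two to five keys, spawned at seeded-random positions in the upper half of the box.
; KillKey tracks removals, then plays one delayed pickup sound per key before opening Finish.
; KillAll destroys remaining keys, then resets and finishes Finish.
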(event `self.ReceiveBeginPlay`
  (`KismetMathLibrary.SeedRandomStream` (`self.RandStream`))
  (`self.Event SpawnKeys` 0))

(event `Event KillKey`
  (params (Key :type "/Game/FirstPersonBP/Blueprints/KeyProjectile Object Reference"))
  (bind _keys (`self.Keys`))
  (bind _returnvalue (`SceneComponent.K2_GetComponentLocation` (`self.DefaultSceneRoot`)))
  (if (!= (`KismetArrayLibrary.Array_Find` _keys Key) -1)
    (`KismetArrayLibrary.Array_RemoveItem` _keys Key)
    (if (== (`KismetArrayLibrary.Array_Length` (`self.Keys`)) 0)
      (`KismetSystemLibrary.Delay` 0.55)
      (switch `int` (`self.Count`)
        (:`Default`
          _)
        (:`2`
          _)
        (:`3`
          (`KismetSystemLibrary.Delay` 0.2 :!label _label)
          (`GameplayStatics.PlaySoundAtLocation` "/Game/Sounds/PickUp_Cue.PickUp_Cue" _returnvalue))
        (:`4`
          (`KismetSystemLibrary.Delay` 0.2 :!label _label_2)
          (`GameplayStatics.PlaySoundAtLocation` "/Game/Sounds/PickUp_Cue.PickUp_Cue" _returnvalue)
          (goto _label))
        (:`5`
          (`KismetSystemLibrary.Delay` 0.2)
          (`GameplayStatics.PlaySoundAtLocation` "/Game/Sounds/PickUp_Cue.PickUp_Cue" _returnvalue)
          (goto _label_2)))
      (`KismetSystemLibrary.Delay` 0.2)
      (`GameplayStatics.PlaySoundAtLocation` "/Game/Sounds/PickUp_Cue.PickUp_Cue" _returnvalue)
      (`KismetSystemLibrary.Delay` 0.2)
      (`GameplayStatics.PlaySoundAtLocation` "/Game/Sounds/PickUp_Cue.PickUp_Cue" _returnvalue)
      (`/Game/Blueprints/FinishButton.Event Open` (`self.Finish`)))))

(event `Event SpawnKeys`
  (params (KeyCount :type Integer))
  (bind _randstream (`self.RandStream`))
  (bind _xbound (`self.XBound`))
  (bind _ybound (`self.YBound`))
  (bind _zbound (`self.ZBound`))
  (switch `int` (`KismetMathLibrary.Clamp` KeyCount 1 4)
    (:`Default`
      (set `self.Count` 2 :!label _label_3))
    (:`0`
      (goto _label_3))
    (:`1`
      (goto _label_3))
    (:`2`
      (set `self.Count` 3))
    (:`3`
      (set `self.Count` 4))
    (:`4`
      (set `self.Count` 5)))
  (`KismetArrayLibrary.Array_Clear` (`self.Keys`))
  (for _ (range 1 (+ (`self.Count`) 1))
    (bind _output_get (set `self.XRand` (`KismetMathLibrary.RandomFloatInRangeFromStream` (* _xbound -1.0) _xbound _randstream)))
    (bind _output_get_2 (set `self.YRand` (`KismetMathLibrary.RandomFloatInRangeFromStream` (* _ybound -1.0) _ybound _randstream)))
    (bind _output_get_3 (set `self.ZRand` (`KismetMathLibrary.RandomFloatInRangeFromStream` _zbound (* _zbound 2.0) _randstream)))
    (bind _returnvalue (`KismetMathLibrary.MakeVector` _output_get _output_get_2 _output_get_3))
    (bind _returnvalue_2 (`|SpawnActorFromClass` "/Game/FirstPersonBP/Blueprints/KeyProjectile.KeyProjectile_C" (`KismetMathLibrary.MakeTransform` (+ _returnvalue (`SceneComponent.K2_GetComponentLocation` (`self.DefaultSceneRoot`))) (`KismetMathLibrary.MakeRotFromX` _returnvalue)) "Undefined" "OverrideRootScale"))
    (set `/Game/FirstPersonBP/Blueprints/KeyProjectile.Controller` self _returnvalue_2)
    (`KismetArrayLibrary.Array_AddUnique` (`self.Keys`) _returnvalue_2)
    (`KismetMathLibrary.SeedRandomStream` (`self.RandStream`))))

(event `Event KillAll`
  (bind _finish (`self.Finish`))
  (for _array_element (`self.Keys`)
    (`self.K2_DestroyActor` _array_element))
  (`/Game/Blueprints/FinishButton.Event Reset` _finish)
  (`/Game/Blueprints/FinishButton.Event Finished` _finish true))

(fn `UserConstructionScript`
  (bind _box (`self.Box`))
  (bind _zbound (`self.ZBound`))
  (`BoxComponent.SetBoxExtent` _box (`KismetMathLibrary.MakeVector` (`self.XBound`) (`self.YBound`) _zbound) true)
  (`SceneComponent.K2_SetRelativeLocation` _box (`KismetMathLibrary.MakeVector` 0.0 0.0 _zbound) false false))